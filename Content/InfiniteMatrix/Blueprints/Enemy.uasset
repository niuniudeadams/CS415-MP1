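; Enemy actor that patrols back and forth, damages the player on contact and can be shot down.
; Tick moves the mesh along Y or Z per MoveLeftRight, with Movearound flipping speed outside a fixed world-coordinate band.
; Mesh overlap with BP_Player removes health, destroys the enemy, then shows a damage HUD or restart.
; Projectile overlap notifies the projectile, destroys the enemy and reports the kill to the player.
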(event OnComponentBeginOverlap(EnemyMesh)
  (params (OverlappedComponent :type Primitive%20Component%20Object%20Reference) (OtherActor :type Actor%20Object%20Reference) (OtherComp :type Primitive%20Component%20Object%20Reference) (OtherBodyIndex :type Integer) (bFromSweep :type Boolean) (SweepResult :type Hit%20Result%20Structure%20%28by%20ref%29))
  (Utilities|FlowControl|Sequence
    (:then_0
      (bind _asbp_player (Utilities|Casting|CastToBP_Player OtherActor))
      (Variables|/Game/InfiniteMatrix/Blueprints/BP_Player.BP_Player_C|SetHealth _asbp_player (- (Variables|/Game/InfiniteMatrix/Blueprints/BP_Player.BP_Player_C|GetHealth _asbp_player) 2e+01))
      (Actor|DestroyActor)
      (if (<= (Variables|/Game/InfiniteMatrix/Blueprints/BP_Player.BP_Player_C|GetHealth _asbp_player) 0.0)
        (Default|DisplayRestart _asbp_player)
        (else
          (bind _returnvalue (UserInterface|CreateWidget "/Game/InfiniteMatrix/UI/HUD_ScreenDamage.HUD_ScreenDamage_C"))
          (UserInterface|Viewport|AddtoViewport _returnvalue 0))))
    (:then_1
      (bind _asprojectile (Utilities|Casting|CastToProjectile OtherActor))
      (Default|HitWallorEnemy _asprojectile)
      (Actor|DestroyActor)
      (bind _asbp_player_2 (Utilities|Casting|CastToBP_Player (Game|Player|GetPlayerPawn 0)))
      (Default|Shootdownenemy _asbp_player_2))))

(event Collision|EventActorBeginOverlap
  (params (OtherActor :type Actor%20Object%20Reference)))

(event EventTick
  (params (DeltaSeconds :type Float%20%28single-precision%29))
  (bind _movespeed (Variables|Default|GetMoveSpeed))
  (bind _enemymesh (Variables|Default|GetEnemyMesh))
  (bind _enemymesh_2 (Variables|Default|GetEnemyMesh))
  (bind _returnvalue (Transformation|GetWorldLocation _enemymesh))
  (bind _returnvalue_2 (* DeltaSeconds _movespeed))
  (if (Variables|Default|GetMoveLeftRight)
    (CallFunction|Movearound (.y _returnvalue))
    (Transformation|AddWorldOffset _enemymesh_2 (Math|Vector|MakeVector 0.0 _returnvalue_2 0.0) false false)
    (else
      (CallFunction|Movearound (.z _returnvalue))
      (Transformation|AddWorldOffset _enemymesh_2 (Math|Vector|MakeVector 0.0 0.0 _returnvalue_2) false false))))

(fn ConstructionScript)

(fn Movearound
  (params (Y%20Or%20Z :type Float%20%28double-precision%29))
  (if (not (Math|Float|InRange(Float) Y%20Or%20Z -2.5e+02 2.5e+02))
    (Variables|Default|SetMoveSpeed (* (Variables|Default|GetMoveSpeed) -1.0))))